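; BP_Player is a player character Blueprint that keeps a record of its default movement friction so it can be reset.
; On BeginPlay it caches the CharacterMovement ground friction and falling lateral friction into base variables.
; Two functions, RestoreBaseGroundFriction and RestoreBaseAirFriction, each write the matching cached value back to the movement component.
; Nothing in these graphs changes friction away from those defaults.
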(event EventBeginPlay
  (bind _charactermovement (Variables|Character|GetCharacterMovement))
  ;[1 1 1] save base friction parameters to restore by functions
  (Variables|Default|SetbaseGroundFriction (Variables|/Script/Engine.CharacterMovementComponent|GetGroundFriction _charactermovement))
  (Variables|Default|SetbaseAirFriction (Variables|/Script/Engine.CharacterMovementComponent|GetFallingLateralFriction _charactermovement)))

(fn ConstructionScript)

(fn RestoreBaseGroundFriction
  (Variables|/Script/Engine.CharacterMovementComponent|SetGroundFriction (Variables|Character|GetCharacterMovement) (Variables|Default|GetbaseGroundFriction)))

(fn RestoreBaseAirFriction
  (Variables|/Script/Engine.CharacterMovementComponent|SetFallingLateralFriction (Variables|Character|GetCharacterMovement) (Variables|Default|GetbaseAirFriction)))