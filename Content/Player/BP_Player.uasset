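; BP_Player is the player character Blueprint, pairing character movement with a BPHealth member for health.
; Incoming damage is deducted through BPHealth, and the current health is printed every tick.
; BeginPlay caches the movement component's ground and falling lateral friction, and two functions restore those values after changes.
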(event EventBeginPlay
  (bind _charactermovement (Variables|Character|GetCharacterMovement))
  ;[1 1 1] save base friction parameters to restore by functions
  (Variables|Private|SetbaseGroundFriction (Variables|/Script/Engine.CharacterMovementComponent|GetGroundFriction _charactermovement))
  (Variables|Private|SetbaseAirFriction (Variables|/Script/Engine.CharacterMovementComponent|GetFallingLateralFriction _charactermovement)))

(event EventTick
  (params (DeltaSeconds :type Float%20%28single-precision%29))
  (Development|PrintString (Utilities|String|ToString(Float) (Default|GetHealth (Variables|Default|GetBP_Health))) true true "(R=0.000000,G=0.660000,B=1.000000,A=1.000000)" 0.0))

(event Game|Damage|EventAnyDamage
  (params (Damage :type Float%20%28single-precision%29) (DamageType :type Damage%20Type%20Object%20Reference) (InstigatedBy :type Controller%20Object%20Reference) (DamageCauser :type Actor%20Object%20Reference))
  (Default|DeductHealth (Variables|Default|GetBP_Health) Damage))

(fn ConstructionScript)

(fn RestoreBaseGroundFriction
  (Variables|/Script/Engine.CharacterMovementComponent|SetGroundFriction (Variables|Character|GetCharacterMovement) (Variables|Private|GetbaseGroundFriction)))

(fn RestoreBaseAirFriction
  (Variables|/Script/Engine.CharacterMovementComponent|SetFallingLateralFriction (Variables|Character|GetCharacterMovement) (Variables|Private|GetbaseAirFriction)))