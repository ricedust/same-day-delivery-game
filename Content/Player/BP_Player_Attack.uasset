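; Player attack component that fires a hitscan attack from its owning BP_Player.
; It casts and caches the owner on BeginPlay, then responds to the IA_Attack input with a short line trace on the Camera channel along the player camera's forward vector.
; Any actor hit receives a fixed amount of damage through ApplyDamage.
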(event Input|EnhancedActionEvents|EnhancedInputActionIA_Attack
  (params (ActionValue :type Boolean) (ElapsedSeconds :type Float%20%28double-precision%29) (TriggeredSeconds :type Float%20%28double-precision%29) (InputAction :type Input%20Action%20Object%20Reference :default "/Game/Player/InputActions/IA_Attack.IA_Attack"))
  (bind _player (Variables|private|Getplayer))
  (bind _camera (Variables|/Game/Player/BP_Player.BP_Player_C|GetCamera _player))
  (bind _returnvalue (Transformation|GetWorldLocation _camera))
  ;[1 1 1] line trace attack
  (bind (_outhit _returnvalue_2) (Collision|LineTraceByChannel _returnvalue (+ _returnvalue (* (Math|Vector|GetForwardVector (Variables|/Game/Player/BP_Player.BP_Player_C|GetCamera (Variables|private|Getplayer))) 1024)) "TraceTypeQuery2" false 0 "None"))
  (if _returnvalue_2
    (Game|Damage|ApplyDamage (.HitActor (Collision|BreakHitResult _outhit)) 1e+01 0 0)))

(event EventBeginPlay
  ;[1 1 1] cache
  (bind _asbp_player (Utilities|Casting|CastToBP_Player (Components|GetOwner)))
  (Variables|private|Setplayer _asbp_player))