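; Player dash component for BP_Player that launches the character along its last movement input when the dash input fires, gated by a cooldown.
; Each dash starts a glide state that swaps in reduced or custom ground and falling lateral friction on the movement component.
; Tick polls velocity and restores the player's base frictions once speed drops to the max walk speed cached at BeginPlay.
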(event Input|EnhancedActionEvents|EnhancedInputActionIA_Dash
  (params (ActionValue :type Boolean) (ElapsedSeconds :type Float%20%28double-precision%29) (TriggeredSeconds :type Float%20%28double-precision%29) (InputAction :type Input%20Action%20Object%20Reference :default "/Game/Player/InputActions/IA_Dash.IA_Dash"))
  (bind _player (Variables|Default|Getplayer))
  (bind _charactermovement (Variables|/Script/Engine.Character|GetCharacterMovement _player))
  ;[1 1 1] attempt dash on input
  (if (not (Variables|Default|GetisDashOnCooldown)) ; ensure we're off cooldown
    ;[1 1 1] actually dash
    (Character|LaunchCharacter (Variables|Default|Getplayer) (* (Class|Pawn|GetLastMovementInputVector (Variables|Default|Getplayer)) (Variables|Default|GetdashSpeed)) false false)
    ;[1 1 1] side effects
    (Utilities|FlowControl|Sequence
      (:then_0
        (Variables|Default|SetisGliding true) ; update isGliding
      )
      (:then_1
        (Variables|Default|SetisDashOnCooldown true) ; start cooldown
        (Utilities|FlowControl|Delay (Variables|Default|GetdashCooldownSeconds))
        (Variables|Default|SetisDashOnCooldown false))
      (:then_2
        (Variables|/Script/Engine.CharacterMovementComponent|SetGroundFriction _charactermovement (Variables|Default|GetglideGroundFriction)) ; apply gliding frictions
        (Variables|/Script/Engine.CharacterMovementComponent|SetFallingLateralFriction _charactermovement (Variables|Default|GetglideAirFriction))))))

(event EventTick
  (params (DeltaSeconds :type Float%20%28single-precision%29))
  ;[1 1 1] poll for when player drops below glide threshold
  (if (and (Variables|Default|GetisGliding) (CallFunction|IsBelowGlideThreshold))
    (Utilities|FlowControl|Sequence
      (:then_0
        (Variables|Default|SetisGliding false))
      (:then_1
        (Default|RestoreBaseGroundFriction (Variables|Default|Getplayer)) ; re-enable normal friction
        (Default|RestoreBaseAirFriction (Variables|Default|Getplayer))))))

(event EventBeginPlay
  ;[1 1 1] cache player reference
  (bind _asbp_player (Utilities|Casting|CastToBP_Player (Components|GetOwner)))
  (Variables|Default|Setplayer _asbp_player)
  ;[1 1 1] set glide speed threshold to max walk speed
  (Variables|Default|SetglideSpeedThreshold (Variables|/Script/Engine.CharacterMovementComponent|GetMaxWalkSpeed (Variables|/Script/Engine.Character|GetCharacterMovement (Variables|Default|Getplayer)))))

(fn IsBelowGlideThreshold
  (return (<= (Math|Vector|VectorLength (Pawn|Components|CharacterMovement|GetLastUpdateVelocity (Variables|/Script/Engine.Character|GetCharacterMovement (Variables|Default|Getplayer)))) (Variables|Default|GetglideSpeedThreshold))))

(fn GetIsGliding
  (return (Variables|Default|GetisGliding)))