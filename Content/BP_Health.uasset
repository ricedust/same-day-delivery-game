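; BP_Health is a health tracker that exposes the current Health value and handles damage to it.
; DeductHealth subtracts an amount, clamps the result at zero, and calls OnHealthDepleted whenever Health is at zero afterward.
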(fn GetHealth
  (return (Variables|Private|Gethealth)))

(fn DeductHealth
  (params (deductBy :type Float%20%28double-precision%29))
  (Variables|Private|Sethealth (Math|Float|Max(Float) (- (Variables|Private|Gethealth) deductBy) 0.0))
  (if (== (Variables|Private|Gethealth) 0.0)
    (Default|CallOnHealthDepleted)))