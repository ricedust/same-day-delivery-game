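; Base enemy Blueprint that takes damage and shows debug information about itself.
; Any damage it receives is passed to its BPHealth component, which deducts it from health.
; Every tick it draws a debug arrow along the capsule's forward vector and prints current health as text above the capsule.
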(event Game|Damage|EventAnyDamage
  (params (Damage :type Float%20%28single-precision%29) (DamageType :type Damage%20Type%20Object%20Reference) (InstigatedBy :type Controller%20Object%20Reference) (DamageCauser :type Actor%20Object%20Reference))
  (Default|DeductHealth (Variables|Default|GetBP_Health) Damage))

(event EventTick
  (params (DeltaSeconds :type Float%20%28single-precision%29))
  (bind _capsulecomponent (Variables|Collision|GetCapsuleComponent))
  (bind _returnvalue (Transformation|GetWorldLocation _capsulecomponent))
  ;[1 1 1] debug facing direction
  (Rendering|Debug|DrawDebugArrow _returnvalue (+ _returnvalue (* (Math|Vector|GetForwardVector (Variables|Collision|GetCapsuleComponent)) 128)) 64.0 "(R=0.000000,G=0.386000,B=0.000000,A=1.000000)" 0.02 4.0)
  ;[1 1 1] debug health
  (Rendering|Debug|DrawDebugString (+ (Transformation|GetWorldLocation (Variables|Collision|GetCapsuleComponent)) "0.000000,0.000000,100.000000") (Utilities|String|ToString(Float) (Default|GetHealth (Variables|Default|GetBP_Health))) 0 "(R=1.000000,G=1.000000,B=1.000000,A=1.000000)"))

(fn ConstructionScript)